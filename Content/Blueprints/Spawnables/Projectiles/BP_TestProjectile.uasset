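; BP_TestProjectile is a test projectile Blueprint that deals damage to what it hits.
; On Hit it prints the hit actor's name, then casts it to BP_Umbrella, falling back to GenericCharacter.
; A successful cast subtracts the truncated ProjectileDamage from that actor's HealthComponent, while other actors take no damage.
; BeginPlay, overlap and Tick events are unused.
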(event EventBeginPlay)

(event Collision|EventActorBeginOverlap
  (params (OtherActor :type Actor%20Object%20Reference)))

(event EventTick
  (params (DeltaSeconds :type Float%20%28single-precision%29)))

(event Collision|EventHit
  (params (MyComp :type Primitive%20Component%20Object%20Reference) (Other :type Actor%20Object%20Reference) (OtherComp :type Primitive%20Component%20Object%20Reference) (bSelfMoved :type Boolean) (HitLocation :type Vector :default "0, 0, 0") (HitNormal :type Vector :default "0, 0, 0") (NormalImpulse :type Vector :default "0, 0, 0") (Hit :type Hit%20Result%20Structure%20%28by%20ref%29))
  ;[0.15 0.04999 0.05148 0.5 30] Making damage on hit.
  (Development|PrintString (Utilities|GetDisplayName Other))
  (bind _asbp_umbrella (Utilities|Casting|CastToBP_Umbrella Other)
    (:then
      (Class|HealthComponent|SubtractHealth (Variables|/Script/LadyUmbrella.Umbrella|GetHealthComponent _asbp_umbrella) (Math|Float|Truncate (Variables|Default|GetProjectileDamage))))
    (:CastFailed
      (bind _asgeneric_character (Utilities|Casting|CastToGenericCharacter Other))
      (Class|HealthComponent|SubtractHealth (Variables|/Script/LadyUmbrella.GenericCharacter|GetHealthComponent _asgeneric_character) (Math|Float|Truncate (Variables|Default|GetProjectileDamage))))))

(fn ConstructionScript)