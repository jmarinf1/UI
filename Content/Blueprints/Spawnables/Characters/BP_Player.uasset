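; Player character Blueprint that carries an umbrella and exposes hooks for an automatic camera system.
; Shortly after BeginPlay, it rescales the umbrella by the inverse of the mesh's world scale, slightly reduced, as a temporary fix for distortion from player scaling.
; Camera hit and close-in events are empty, and the camera state and modifier calls are unwired.
; SpawnUmbrellaInHand is also empty, with disconnected socket-attach logic.
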(event EventBeginPlay
  (bind _returnvalue (Class|PlayerCharacter|GetUmbrella))
  (bind _mesh (Variables|Character|GetMesh))
  (bind _returnvalue_2 (Transformation|GetWorldScale _mesh))
  ;[0.15 0.15 0.15 0.5] Since the player is scaled, the umbrella is scaled too, and isn't circular, this helps but will have to be deleted
  (Utilities|FlowControl|Delay 0.2)
  (Utilities|IsValid _returnvalue
    (:Is%20Valid
      (Transformation|SetActorRelativeScale3D _returnvalue (* (Math|Vector|MakeVector (/ 1.0 (.x _returnvalue_2)) (/ 1.0 (.y _returnvalue_2)) (/ 1.0 (.z _returnvalue_2))) 0.9)))))

(event EventOnCameraSideHit
  (params (HitLeft :type Boolean))
  ;[0.0203 0.07179 0.15 0.5] Automatic Camera Functions
  ;;[0.149 0.02891 0.0215 0.502] Events
)

(event EventOnCameraClosein
  ;[0.0203 0.07179 0.15 0.5] Automatic Camera Functions
  ;;[0.149 0.02891 0.0215 0.502] Events
)

(event EventOnCameraBackHit
  ;[0.0203 0.07179 0.15 0.5] Automatic Camera Functions
  ;;[0.149 0.02891 0.0215 0.502] Events
)

(fn ConstructionScript)

(fn SpawnUmbrellainHand)