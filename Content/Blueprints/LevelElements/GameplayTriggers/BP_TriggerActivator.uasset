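; Trigger volume that swaps two tagged groups of level actors when something overlaps its Box.
; On BeginPlay it hides and disables collision on "ActivablePorTrigger" actors, while showing and enabling those tagged "LaserTrigger".
; Any overlap with the Box inverts both groups, with no filter on the overlapping actor and no logic to switch back.
; Targets are found level-wide by actor tag rather than through assigned references.
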(event OnComponentBeginOverlap(Box)
  (params (OverlappedComponent :type Primitive%20Component%20Object%20Reference) (OtherActor :type Actor%20Object%20Reference) (OtherComp :type Primitive%20Component%20Object%20Reference) (OtherBodyIndex :type Integer) (bFromSweep :type Boolean) (SweepResult :type Hit%20Result%20Structure%20%28by%20ref%29))
  (Utilities|FlowControl|Sequence
    (:then_0
      (bind _outactors (Actor|GetAllActorswithTag "ActivablePorTrigger"))
      (Rendering|SetActorHiddenInGame _outactors false)
      (Collision|SetActorEnableCollision _outactors true))
    (:then_1
      (bind _outactors_2 (Actor|GetAllActorswithTag "LaserTrigger"))
      (Rendering|SetActorHiddenInGame _outactors_2 true)
      (Collision|SetActorEnableCollision _outactors_2 false))))

(event EventBeginPlay
  (Utilities|FlowControl|Sequence
    (:then_0
      (bind _outactors (Actor|GetAllActorswithTag "ActivablePorTrigger"))
      (Rendering|SetActorHiddenInGame _outactors true)
      (Collision|SetActorEnableCollision _outactors false))
    (:then_1
      (bind _outactors_2 (Actor|GetAllActorswithTag "LaserTrigger"))
      (Rendering|SetActorHiddenInGame _outactors_2 false)
      (Collision|SetActorEnableCollision _outactors_2 true))))

(event Collision|EventActorBeginOverlap
  (params (OtherActor :type Actor%20Object%20Reference)))

(event EventTick
  (params (DeltaSeconds :type Float%20%28single-precision%29)))

(fn ConstructionScript)