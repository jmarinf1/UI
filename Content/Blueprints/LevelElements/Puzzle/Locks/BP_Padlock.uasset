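; BP_Padlock is a puzzle lock actor that opens when its reacted delegate fires.
; On BeginPlay it binds React, which switches the padlock state and prints a debug string.
; ChangePadlockState swaps the mesh from a state-to-mesh map and calls the lock-open dispatcher.
; It then enables physics simulation and collision on the mesh, regardless of the state passed in.
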(event Custom|React
  (CallFunction|ChangePadlockState "NewEnumerator1")
  (Development|PrintString "Hello"))

(event EventBeginPlay
  (EventDispatchers|BindEventtoOnReactedDelegate self (delegate Custom|React)))

(event Collision|EventActorBeginOverlap
  (params (OtherActor :type Actor%20Object%20Reference)))

(event EventTick
  (params (DeltaSeconds :type Float%20%28single-precision%29)))

(fn ConstructionScript
  (|CallParentFunction))

(fn ChangePadlockState
  (params (New%20State :type E_PadlockStates%20Enum :default "NewEnumerator0"))
  (bind _objectmesh (Variables|Default|GetObjectMesh))
  (bind _output_get (Variables|Default|SetCurrentState New%20State))
  (Components|StaticMesh|SetStaticMesh (Variables|Default|GetObjectMesh) (.Value (Utilities|Map|Find (Variables|Default|GetPadlockMeshes) _output_get)))
  (Default|CallOnLockOpen)
  (Physics|SetSimulatePhysics _objectmesh true)
  (Collision|SetCollisionEnabled _objectmesh "QueryAndPhysics"))