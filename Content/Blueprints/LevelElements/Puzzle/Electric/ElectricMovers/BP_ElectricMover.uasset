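; BP_ElectricMover is an electric puzzle element that relocates itself by a configurable offset when electrified.
; On BeginPlay it stores its transform and adds RelativeOffset to the location, unrotated, to get the target.
; OnElectrified snaps the actor there instantly, with no interpolation or sweep; the return-to-initial function is an empty stub.
; The construction script places DebugPlatform at MovingPlatform's relative location plus the offset as a destination preview.
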(event EventBeginPlay
  (CallFunction|InitializeTransform)
  (CallFunction|CalculateTargetPosition))

(event Collision|EventActorBeginOverlap
  (params (OtherActor :type Actor%20Object%20Reference)))

(event EventTick
  (params (DeltaSeconds :type Float%20%28single-precision%29)))

(event EventOnElectrified
  (CallFunction|MoveElementtoTargetPosition))

(fn ConstructionScript
  (Transformation|SetRelativeLocation (Variables|Default|GetDebugPlatform) (+ (.location (Transformation|GetRelativeTransform (Variables|Default|GetMovingPlatform))) (Variables|Default|GetRelativeOffset)) false false))

(fn InitializeTransform
  (Variables|Default|SetInitialTransform (Transformation|GetActorTransform self)))

(fn MoveElementtoTargetPosition
  (Transformation|SetActorLocation (.location (Variables|Default|GetTargetTransform)) false false))

(fn MoveElementtoInitialPosition)

(fn CalculateTargetPosition
  (bind _initialtransform (Variables|Default|GetInitialTransform))
  (Variables|Default|SetTargetTransform (Math|Transform|MakeTransform (+ (.location _initialtransform) (Variables|Default|GetRelativeOffset)) (.rotation _initialtransform) (.scale _initialtransform))))