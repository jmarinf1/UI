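; Electric puzzle element actor that rotates when it receives the OnElectrified event.
; Each activation combines the current actor rotation with the FinalTransform rotation and sets it instantly as relative rotation, so repeated triggers accumulate.
; The construction script applies FinalTransform to RotableElementDebug as a preview.
; InitialTransform is cached on BeginPlay but unused here, and UnrotateElement is an empty stub.
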(event EventBeginPlay
  (CallFunction|InitializeTransform))

(event Collision|EventActorBeginOverlap
  (params (OtherActor :type Actor%20Object%20Reference)))

(event EventTick
  (params (DeltaSeconds :type Float%20%28single-precision%29)))

(event EventOnElectrified
  (CallFunction|RotateElement))

(fn ConstructionScript
  (Transformation|SetRelativeTransform (Variables|Default|GetRotableElementDebug) (Variables|Default|GetFinalTransform) false false))

(fn InitializeTransform
  (Variables|Default|SetInitialTransform (Transformation|GetActorTransform self)))

(fn RotateElement
  (bind _self self)
  (bind _finaltransform (Variables|Default|GetFinalTransform))
  (Transformation|SetActorRelativeRotation _self (Math|Rotator|CombineRotators (Transformation|GetActorRotation _self) (Math|Rotator|MakeRotator (.roll (.rotation _finaltransform)) (.pitch (.rotation _finaltransform)) (.yaw (.rotation _finaltransform))))))

(fn UnrotateElement)