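; Double-leaf swinging variant of an automatic door, kept in a folder marked DONT_USE.
; The construction script builds two mirrored DoorParts from one mesh, each with closed and open transforms, using the left and right opening angles as yaw.
; It also rotates the two open-position components to those angles, then runs the parent construction script with the filled DoorParts array.
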(fn ConstructionScript
  (bind _array (Utilities|Array|MakeArray))
  (bind _doormesh (Variables|Default|GetDoorMesh))
  (Transformation|SetRelativeRotation (Variables|Default|GetRightOpenPosition) (Math|Rotator|MakeRotator 0.0 0.0 (* (Variables|Default|GetRightDoorOpening) -1.0)) false false)
  (Transformation|SetRelativeRotation (Variables|Default|GetLeftOpenPosition) (Math|Rotator|MakeRotator 0.0 0.0 (- (Variables|Default|GetLeftDoorOpening) 1.8e+02)) false false)
  (Variables|Default|SetDoorParts (Utilities|Array|MakeArray (Utilities|Struct|MakeF_DoorParts _doormesh _array (Math|Transform|MakeTransform "-100.000000, 0, 0" "0,-180.000000, 0") (Math|Transform|MakeTransform "-100.000000, 0, 0" (Math|Rotator|MakeRotator 0.0 0.0 (- (Variables|Default|GetLeftDoorOpening) 1.8e+02)))) (Utilities|Struct|MakeF_DoorParts _doormesh _array (Math|Transform|MakeTransform "100.000000,0.000000, 0") (Math|Transform|MakeTransform "100.000000, 0, 0" (Math|Rotator|MakeRotator 0.0 0.0 (* (Variables|Default|GetRightDoorOpening) -1.0))))))
  (|CallParentFunction))