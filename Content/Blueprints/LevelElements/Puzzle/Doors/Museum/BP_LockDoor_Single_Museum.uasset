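; Single locked museum door puzzle element that triggers a security system when its padlock reacts.
; On BeginPlay, after the parent logic runs, it binds SecuritySystem to the reacted delegate of PadlockReference.
; SecuritySystem finds every actor tagged "ActivablePorTrigger", then unhides it and enables its collision, so the revealed actors are chosen purely by tag.
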(event Custom|SecuritySystem
  (bind _outactors (Actor|GetAllActorswithTag "ActivablePorTrigger"))
  (Rendering|SetActorHiddenInGame _outactors false)
  (Collision|SetActorEnableCollision _outactors true))

(event EventBeginPlay
  (|CallParentFunction)
  (EventDispatchers|BindEventtoOnReactedDelegate (Variables|Default|GetPadlock%20Reference) (delegate Custom|SecuritySystem)))

(event Collision|EventActorBeginOverlap
  (params (OtherActor :type Actor%20Object%20Reference))
  (|CallParentFunction OtherActor) ; This node is disabled and will not be called.\nDrag off pins to build functionality.
)

(event EventTick
  (params (DeltaSeconds :type Float%20%28single-precision%29))
  (|CallParentFunction DeltaSeconds) ; This node is disabled and will not be called.\nDrag off pins to build functionality.
)

(fn ConstructionScript
  (|CallParentFunction))