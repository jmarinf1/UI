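; Double-door variant of a lock door puzzle element, built on a parent Blueprint with no event logic of its own.
; The construction script turns the left and right opening angles into mirrored yaw rotations on the two open-position components.
; It fills the DoorParts array with each leaf's mesh and fixed-hinge closed and open transforms, then runs the parent construction script.
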(event EventBeginPlay
  (|CallParentFunction) ; This node is disabled and will not be called.\nDrag off pins to build functionality.
)

(event Collision|EventActorBeginOverlap
  (params (OtherActor :type Actor%20Object%20Reference))
  (|CallParentFunction OtherActor) ; This node is disabled and will not be called.\nDrag off pins to build functionality.
)

(event EventTick
  (params (DeltaSeconds :type Float%20%28single-precision%29))
  (|CallParentFunction DeltaSeconds) ; This node is disabled and will not be called.\nDrag off pins to build functionality.
)

(fn ConstructionScript
  (bind _array (Utilities|Array|MakeArray))
  (Transformation|SetRelativeRotation (Variables|Default|GetRightOpenPosition) (Math|Rotator|MakeRotator 0.0 0.0 (* (Variables|Default|GetRightDoorOpening) -1.0)) false false)
  (Transformation|SetRelativeRotation (Variables|Default|GetLeftOpenPosition) (Math|Rotator|MakeRotator 0.0 0.0 (- (Variables|Default|GetLeftDoorOpening) 0.0)) false false)
  (Variables|Default|SetDoorParts (Utilities|Array|MakeArray (Utilities|Struct|MakeF_DoorParts (Variables|Default|GetDoorMesh_Left) _array (Math|Transform|MakeTransform "50.000000,-10.000000,10.000000") (Math|Transform|MakeTransform "50.000000,-10.000000,10.000000" (Math|Rotator|MakeRotator 0.0 0.0 (- (Variables|Default|GetLeftDoorOpening) 0.0)))) (Utilities|Struct|MakeF_DoorParts (Variables|Default|GetDoorMesh_Right) _array (Math|Transform|MakeTransform "350.000000,-10.000000,10.000000") (Math|Transform|MakeTransform "350.000000,-10.000000,10.000000" (Math|Rotator|MakeRotator 0.0 0.0 (* (Variables|Default|GetRightDoorOpening) -1.0))))))
  (|CallParentFunction))