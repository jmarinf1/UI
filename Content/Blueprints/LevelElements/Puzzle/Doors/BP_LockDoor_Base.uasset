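; Base puzzle door that can start locked behind a padlock and opens when that lock is opened.
; On BeginPlay, a locked door caches its BP_Padlock child actor and listens for its open event, while an unlocked door destroys the padlock component.
; Unlocking enables TriggerActive and marks the door open.
; Lock state is shown by swapping the locked or unlocked material across all door components.
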(event Custom|UnlockDoor
  (Variables|Default|SetTriggerActive true)
  (Variables|Default|SetDoorIsOpen true)
  (CallFunction|UpdateDoorMaterials (Variables|Default|GetUnlockedMaterial)))

(event EventBeginPlay
  (bind _padlock_reference (Variables|Default|GetPadlock%20Reference))
  (CallFunction|InitializeLockState)
  (if (!= _padlock_reference 0)
    (EventDispatchers|BindEventtoOnLockOpen _padlock_reference (delegate Custom|UnlockDoor))))

(event Collision|EventActorBeginOverlap
  (params (OtherActor :type Actor%20Object%20Reference)))

(event EventTick
  (params (DeltaSeconds :type Float%20%28single-precision%29))
  (|CallParentFunction DeltaSeconds) ; This node is disabled and will not be called.\nDrag off pins to build functionality.
)

(fn ConstructionScript
  (|CallParentFunction))

(fn InitializeLockState
  (bind _bp_padlock (Variables|Default|GetBP_Padlock))
  (bind _startlocked (Variables|Default|GetStartLocked))
  (Variables|Default|SetTriggerActive (not _startlocked))
  (if _startlocked
    ;[0.02606 0.15 0.03368 0.5] If the door is locked we Set the padlock reference to later listen to the open event
    (bind _asbp_padlock (Utilities|Casting|CastToBP_Padlock (Variables|/Script/Engine.ChildActorComponent|GetChildActor _bp_padlock)))
    (Variables|Default|SetPadlock%20Reference _asbp_padlock)
    (CallFunction|UpdateDoorMaterials (Variables|Default|GetLockedMaterial))
    (else
      ;[0.15 0.0234 0.02638 0.5] If the door is not locked, we don't need the lock so we destroy it
      (Components|DestroyComponent _bp_padlock)
      (CallFunction|UpdateDoorMaterials (Variables|Default|GetUnlockedMaterial))))
  (return))

(fn UpdateDoorMaterials
  (params (NewMaterial :type Material%20Instance%20Object%20Reference))
  (for _array_element (Variables|Default|GetDoorsComponnent)
    (Rendering|Material|SetMaterial _array_element 0 NewMaterial)))