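; BP_LockedDoorExample is an example puzzle door that opens when a linked falling element runs out of simulation time.
; Each tick it casts its FallingElement child actor and checks whether SimulationSeconds has reached zero.
; When it has, the left and right hinges snap 90 degrees in opposite directions, and an Open flag keeps this from repeating.
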(event EventTick
  (params (DeltaSeconds :type Float%20%28single-precision%29))
  (bind _asfalling_element (Utilities|Casting|CastToFallingElement (Variables|/Script/Engine.ChildActorComponent|GetChildActor (Variables|Default|GetFallingElement))))
  (if (and (<= (Variables|/Script/LadyUmbrella.FallingElement|GetSimulationSeconds _asfalling_element) 0.0) (not (Variables|Default|GetOpen)))
    (Transformation|AddLocalRotation (Variables|Default|GetHingeRight) "0.000000,90.000000,0.000000" false false)
    (Transformation|AddLocalRotation (Variables|Default|GetHingeLeft) "0.000000,-90.000000,0.000000" false false)
    (Variables|Default|SetOpen true)))

(fn ConstructionScript)