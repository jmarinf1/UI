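; Single-leaf lock door for puzzle levels, configuring a parent door Blueprint that receives all of its runtime logic.
; The construction script fills DoorParts with one entry: DoorMesh with closed and open transforms at the same location, the open one yawed by negated RightDoorOpening.
; It also rotates the RightOpenPosition component to that yaw, so the open pose follows the variable.
; BeginPlay only calls the parent.
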(event EventBeginPlay
  (|CallParentFunction))

(event Collision|EventActorBeginOverlap
  (params (OtherActor :type Actor%20Object%20Reference))
  (|CallParentFunction OtherActor) ; This node is disabled and will not be called.\nDrag off pins to build functionality.
)

(event EventTick
  (params (DeltaSeconds :type Float%20%28single-precision%29)))

(fn ConstructionScript
  (Transformation|SetRelativeRotation (Variables|Default|GetRightOpenPosition) (Math|Rotator|MakeRotator 0.0 0.0 (* (Variables|Default|GetRightDoorOpening) -1.0)) false false)
  (Variables|Default|SetDoorParts (Utilities|Array|MakeArray (Utilities|Struct|MakeF_DoorParts (Variables|Default|GetDoorMesh) (Utilities|Array|MakeArray) (Math|Transform|MakeTransform "175.000000,-10.000000,10.000000") (Math|Transform|MakeTransform "175.000000,-10.000000,10.000000" (Math|Rotator|MakeRotator 0.0 0.0 (* (Variables|Default|GetRightDoorOpening) -1.0))))))
  (|CallParentFunction))