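; BP_NoteComment_AutoAdjustment is a level design note actor that displays a title and description with a pointer to an end point.
; Its construction script sets both texts, passing the description through WrapText, which builds lines limited by MaxCharsPerLine.
; It also moves a cube to EndPoint, then rotates the spline mesh toward it and scales the mesh's end position from the distance, so the pointer adjusts automatically.
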(event EventBeginPlay)

(event Collision|EventActorBeginOverlap
  (params (OtherActor :type Actor%20Object%20Reference)))

(event EventTick
  (params (DeltaSeconds :type Float%20%28single-precision%29)))

(fn ConstructionScript
  (bind _splinemesh (Variables|Default|GetSplineMesh))
  (bind _endpointloccube (Variables|Default|GetEndPointLocCube))
  (bind _returnvalue (Transformation|GetWorldLocation _endpointloccube))
  (bind _returnvalue_2 (Transformation|GetWorldLocation _splinemesh))
  (Rendering|Components|TextRender|SetText (Variables|Default|GetTitleText) (Variables|Default|GetTitle))
  (bind _resultstring (CallFunction|WrapText (Variables|Default|GetDescription)))
  (Rendering|Components|TextRender|SetText (Variables|Default|GetDescriptionText) _resultstring)
  (Transformation|SetRelativeLocation (Variables|Default|GetEndPointLocCube) (Variables|Default|GetEndPoint) false false)
  (Transformation|SetWorldRotation _splinemesh (Math|Rotator|FindLookatRotation _returnvalue_2 _returnvalue) false false)
  (SplineMesh|SetEndPosition _splinemesh (Math|Vector|MakeVector (* (Math|Vector|Distance(Vector) _returnvalue_2 _returnvalue) 2e+01) 0.0 0.0) true))

(fn WrapText
  (params (InputText :type Text))
  (bind _output_get (LocalVariables|SetInput%20Text InputText))
  (for _array_element (Utilities|String|ParseIntoArray (Utilities|String|ToString(Text) _output_get) " ")
    (if (Utilities|Text|TextIsEmpty (Variables|Default|GetCurrentLine))
      (Variables|Default|SetSeparator "")
      (else
        (Variables|Default|SetSeparator " ")))
    (if (> (Utilities|String|Len (Utilities|String|Append (Utilities|String|ToString(Text) (Variables|Default|GetCurrentLine)) (Utilities|String|ToString(Text) (Variables|Default|GetSeparator)) _array_element)) (Variables|Default|GetMaxCharsPerLine))
      (Variables|Default|SetResultString (Utilities|Text|ToText(String) (Utilities|String|Append (Utilities|String|ToString(Text) (Variables|Default|GetResultString)) (Utilities|String|ToString(Text) (Variables|Default|GetCurrentLine)) (Utilities|String|ToString(Text) (Utilities|Text|MakeLiteralText " 
")))))
      (Variables|Default|SetCurrentLine (Utilities|Text|ToText(String) _array_element))
      (else
        (Variables|Default|SetCurrentLine (Utilities|Text|ToText(String) (Utilities|String|Append (Utilities|String|ToString(Text) (Variables|Default|GetCurrentLine)) (Utilities|String|ToString(Text) (Variables|Default|GetSeparator)) _array_element))))))
  (return (Utilities|Text|ToText(String) (Utilities|String|Append (Utilities|String|ToString(Text) (Variables|Default|GetResultString)) (Utilities|String|ToString(Text) (Variables|Default|GetCurrentLine))))))