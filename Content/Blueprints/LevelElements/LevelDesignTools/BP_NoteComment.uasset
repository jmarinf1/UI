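; BP_NoteComment is a level design annotation actor that shows a title and description with a pointer toward a chosen location.
; The construction script pushes Title and Description into text components and moves an end point cube to the EndPoint offset.
; It then rotates a spline mesh toward the cube and scales the mesh's end position by their distance to form a connecting line.
; The event graph has no active logic.
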(event EventBeginPlay)

(event Collision|EventActorBeginOverlap
  (params (OtherActor :type Actor%20Object%20Reference)))

(event EventTick
  (params (DeltaSeconds :type Float%20%28single-precision%29)))

(fn ConstructionScript
  (bind _splinemesh (Variables|Default|GetSplineMesh))
  (bind _endpointloccube (Variables|Default|GetEndPointLocCube))
  (bind _returnvalue (Transformation|GetWorldLocation _endpointloccube))
  (bind _returnvalue_2 (Transformation|GetWorldLocation _splinemesh))
  (Rendering|Components|TextRender|SetText (Variables|Default|GetTitleText) (Variables|Default|GetTitle))
  (Rendering|Components|TextRender|SetText (Variables|Default|GetDescriptionText) (Variables|Default|GetDescription))
  (Transformation|SetRelativeLocation (Variables|Default|GetEndPointLocCube) (Variables|Default|GetEndPoint) false false)
  (Transformation|SetWorldRotation _splinemesh (Math|Rotator|FindLookatRotation _returnvalue_2 _returnvalue) false false)
  (SplineMesh|SetEndPosition _splinemesh (Math|Vector|MakeVector (* (Math|Vector|Distance(Vector) _returnvalue_2 _returnvalue) 2e+01) 0.0 0.0) true))