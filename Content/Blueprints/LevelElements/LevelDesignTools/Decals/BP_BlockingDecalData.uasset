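; Level design tool Blueprint that holds a blocking decal's appearance settings and applies them to the decal's material.
; SetDecalMaterialParameters stores the settings struct, then writes texture, color, opacity mode and transform values to the decal's dynamic material instance, if it has one.
; Texture scale is divided by the ratio of decal size to decal region, and offset is multiplied by the unadjusted scale.
; UpdateDecalMaterialParameters reapplies the stored settings.
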(fn SetDecalMaterialParameters
  (params (Parameters_Struct :type F%20Blocking%20Decal%20Material%20Parameters%20Structure%20%28by%20ref%29))
  (bind _decal_region (Variables|Default|GetDecal%20Region))
  (bind _decal_size (Variables|Default|GetDecal%20Size))
  (bind (_x _y) (Math|Vector2D|BreakVector2D _decal_region))
  (bind (_x_2 _y_2) (Math|Vector2D|BreakVector2D _decal_size))
  (Variables|Default|SetDecal%20Parameters Parameters_Struct)
  (bind _asmaterial_instance_dynamic (Utilities|Casting|CastToMaterialInstanceDynamic (Class|DecalComponent|GetDecalMaterial (Variables|Default|GetDecalComponent))))
  (LocalVariables|SetCurrentMaterial _asmaterial_instance_dynamic)
  (Rendering|Material|SetScalarParameterValue (LocalVariables|GetCurrentMaterial) "UseTexture" (Math|Conversions|ToFloat(Boolean) (.UseTexture (Utilities|Struct|BreakF_BlockingDecalMaterialParameters (Variables|Default|GetDecal%20Parameters)))) :!class /Script/Engine.MaterialInstanceDynamic)
  (Rendering|Material|SetTextureParameterValue (LocalVariables|GetCurrentMaterial) "Texture" (.Texture (Utilities|Struct|BreakF_BlockingDecalMaterialParameters (Variables|Default|GetDecal%20Parameters))))
  (Rendering|Material|SetVectorParameterValue (LocalVariables|GetCurrentMaterial) "Color" (.Color (Utilities|Struct|BreakF_BlockingDecalMaterialParameters (Variables|Default|GetDecal%20Parameters))) :!class /Script/Engine.MaterialInstanceDynamic)
  (Rendering|Material|SetScalarParameterValue (LocalVariables|GetCurrentMaterial) "TextureColorForOpacity" (Math|Conversions|ToFloat(Boolean) (.TextureColorForOpacity (Utilities|Struct|BreakF_BlockingDecalMaterialParameters (Variables|Default|GetDecal%20Parameters)))) :!class /Script/Engine.MaterialInstanceDynamic)
  (Rendering|Material|SetScalarParameterValue (LocalVariables|GetCurrentMaterial) "ZRotation" (.TextureRotation (Utilities|Struct|BreakF_BlockingDecalMaterialParameters (Variables|Default|GetDecal%20Parameters))) :!class /Script/Engine.MaterialInstanceDynamic)
  (Rendering|Material|SetScalarParameterValue (LocalVariables|GetCurrentMaterial) "XScale" (/ (.X (Math|Vector2D|BreakVector2D (.TextureScale (Utilities|Struct|BreakF_BlockingDecalMaterialParameters (Variables|Default|GetDecal%20Parameters))))) (/ _x_2 _x)) :!class /Script/Engine.MaterialInstanceDynamic)
  (Rendering|Material|SetScalarParameterValue (LocalVariables|GetCurrentMaterial) "YScale" (/ (.Y (Math|Vector2D|BreakVector2D (.TextureScale (Utilities|Struct|BreakF_BlockingDecalMaterialParameters (Variables|Default|GetDecal%20Parameters))))) (/ _y_2 _y)) :!class /Script/Engine.MaterialInstanceDynamic)
  (Rendering|Material|SetScalarParameterValue (LocalVariables|GetCurrentMaterial) "YLocation" (* (.Y (Math|Vector2D|BreakVector2D (.TextureScale (Utilities|Struct|BreakF_BlockingDecalMaterialParameters (Variables|Default|GetDecal%20Parameters))))) (.Y (Math|Vector2D|BreakVector2D (.TextureOffset (Utilities|Struct|BreakF_BlockingDecalMaterialParameters (Variables|Default|GetDecal%20Parameters)))))) :!class /Script/Engine.MaterialInstanceDynamic)
  (Rendering|Material|SetScalarParameterValue (LocalVariables|GetCurrentMaterial) "XLocation" (* (.X (Math|Vector2D|BreakVector2D (.TextureScale (Utilities|Struct|BreakF_BlockingDecalMaterialParameters (Variables|Default|GetDecal%20Parameters))))) (.X (Math|Vector2D|BreakVector2D (.TextureOffset (Utilities|Struct|BreakF_BlockingDecalMaterialParameters (Variables|Default|GetDecal%20Parameters)))))) :!class /Script/Engine.MaterialInstanceDynamic))

(fn UpdateDecalMaterialParameters
  (CallFunction|SetDecalMaterialParameters (Variables|Default|GetDecal%20Parameters)))