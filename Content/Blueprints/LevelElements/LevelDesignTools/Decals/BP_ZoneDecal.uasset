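; BP_ZoneDecal is a level design tool that outlines a polygonal zone with decals, built entirely in the construction script.
; It places a configurable number of corners around the actor, scaled by decal size and offset by a zone rotation.
; Each side decal is derived from adjacent corners, using their midpoint and half their distance as length.
; Corner decals sort above sides and can optionally rotate with their corner.
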(event EventBeginPlay
  (|CallParentFunction) ; This node is disabled and will not be called.\nDrag off pins to build functionality.
)

(event Collision|EventActorBeginOverlap
  (params (OtherActor :type Actor%20Object%20Reference)))

(event EventTick
  (params (DeltaSeconds :type Float%20%28single-precision%29))
  (|CallParentFunction DeltaSeconds) ; This node is disabled and will not be called.\nDrag off pins to build functionality.
)

(fn ConstructionScript
  (bind _decal_side_size (Variables|Default|GetDecal%20Side%20Size))
  (bind _decal_size (Variables|Default|GetDecal%20Size))
  (bind _decal_corner_size (Variables|Default|GetDecal%20Corner%20Size))
  (bind _corner_transform (Variables|Default|GetCorner%20Transform))
  (bind (_x _y) (Math|Vector2D|BreakVector2D _decal_size))
  (|CallParentFunction)
  (for _index (range 0 (Variables|Default|GetNumber%20of%20Sides))
    (if (!= _index 0)
      ;[1 1 1] Create corner points
      (Utilities|Array|Add (Variables|Default|GetCorner%20Transform) (Math|Transform|ComposeTransforms (Math|Transform|MakeTransform (* (Math|Vector|RotateVector (Math|Vector|MakeVector (Math|Float|SelectFloat (Math|Vector2D|Vector2DLength "(X=1.000000,Y=1.000000)") 1.0 (Variables|Default|GetUse%20Decal%20Corner%20As%20Distance)) 0.0 0.0) (Math|Rotator|MakeRotator 0.0 0.0 (+ (* (/ (Math|Conversions|ToFloat(Integer) _index) (Variables|Default|GetNumber%20of%20Sides)) 3.6e+02) (Variables|Default|GetZone%20Rotation%20Offset)))) (Math|Vector|MakeVector _x _y 0.0)) (Math|Rotator|MakeRotator 0.0 0.0 (+ (* (/ (Math|Conversions|ToFloat(Integer) _index) (Variables|Default|GetNumber%20of%20Sides)) 3.6e+02) (Variables|Default|GetZone%20Rotation%20Offset)))) (Transformation|GetActorTransform)))))
  (for (_array_element _array_index) (Variables|Default|GetCorner%20Transform)
    (if (== _array_index 0)
      ;[1 1 1] Create corner points
      (LocalVariables|SetTransform (CallFunction|GetSideDecalTransform _array_element (Utilities|Array|Get(acopy) _corner_transform (Utilities|Array|LastIndex _corner_transform))))
      (else
        (LocalVariables|SetTransform (CallFunction|GetSideDecalTransform _array_element (Utilities|Array|Get(acopy) (Variables|Default|GetCorner%20Transform) (+ _array_index -1))))))
    (Utilities|Array|Add (Variables|Default|GetSides%20Transform) (LocalVariables|GetTransform)))
  (Utilities|FlowControl|Sequence
    (:then_0)
    (:then_1)
    (:then_2
      (for _array_element_2 (Variables|Default|GetCorner%20Transform)
        (bind _return_value (CallFunction|CreateDecal (Variables|Default|GetDecal%20Height) _decal_corner_size _decal_corner_size (Variables|Default|GetCorner%20Material) (Variables|Default|GetCorner%20Mat%20Params) (+ (Variables|Default|GetDecals%20Short%20Order) 1)))
        (Transformation|SetWorldLocation (Variables|/Game/Blueprints/LevelElements/LevelDesignTools/Decals/BP_BlockingDecalData.BP_BlockingDecalData_C|GetDecalRootComponent _return_value) (.Location (Math|Transform|BreakTransform _array_element_2)) false true)
        (if (Variables|Default|GetOriant%20Corners)
          (Transformation|AddRelativeRotation (Variables|/Game/Blueprints/LevelElements/LevelDesignTools/Decals/BP_BlockingDecalData.BP_BlockingDecalData_C|GetDecalRootComponent _return_value) (.Rotation (Math|Transform|BreakTransform _array_element_2)) false false)))
      (for _array_element_3 (Variables|Default|GetSides%20Transform)
        (bind _return_value_2 (CallFunction|CreateDecal (Variables|Default|GetDecal%20Height) (Math|Vector2D|MakeVector2D (.Y (Math|Vector|BreakVector (.Scale (Math|Transform|BreakTransform _array_element_3)))) (.Z (Math|Vector|BreakVector (.Scale (Math|Transform|BreakTransform _array_element_3))))) (Math|Vector2D|MakeVector2D _decal_side_size _decal_side_size) (Variables|Default|GetSide%20Material) (Variables|Default|GetSide%20Mat%20Params) (Variables|Default|GetDecals%20Short%20Order)))
        (Transformation|SetWorldLocation (Variables|/Game/Blueprints/LevelElements/LevelDesignTools/Decals/BP_BlockingDecalData.BP_BlockingDecalData_C|GetDecalRootComponent _return_value_2) (.Location (Math|Transform|BreakTransform _array_element_3)) false true)
        (Transformation|AddRelativeRotation (Variables|/Game/Blueprints/LevelElements/LevelDesignTools/Decals/BP_BlockingDecalData.BP_BlockingDecalData_C|GetDecalRootComponent _return_value_2) (.Rotation (Math|Transform|BreakTransform _array_element_3)) false false)))))

(fn GetSideDecalTransform
  (params (A :type Transform%20%28by%20ref%29) (B :type Transform%20%28by%20ref%29))
  (bind _returnvalue (Math|Transform|Lerp(Transform) A B 0.5))
  (bind (_location _rotation) (Math|Transform|BreakTransform _returnvalue))
  (return (Math|Transform|MakeTransform _location (Math|Rotator|CombineRotators "0,90.000000, 0" _rotation) (Math|Vector|MakeVector 0.0 (* (Math|Vector|VectorLength (- (.Location (Math|Transform|BreakTransform A)) (.Location (Math|Transform|BreakTransform B)))) 0.5) (Variables|Default|GetDecal%20Side%20Size)))))