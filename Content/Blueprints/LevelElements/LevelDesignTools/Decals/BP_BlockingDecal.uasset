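; BP_BlockingDecal is a level design actor that creates and manages decals, with a DecalZone box sized from its decal size and height.
; CreateDecal builds a BP_BlockingDecalData object per decal, holding a downward-pitched, scaled decal component under its own scene root with a dynamic material instance.
; The construction script only resizes the box, while UpdateDecal also refreshes material parameters across every stored decal.
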(event EventBeginPlay)

(event Collision|EventActorBeginOverlap
  (params (OtherActor :type Actor%20Object%20Reference)))

(event EventTick
  (params (DeltaSeconds :type Float%20%28single-precision%29)))

(fn ConstructionScript
  (CallFunction|UpdateDecalZone))

(fn CreateDecal
  (params (In%20Decal%20Height :type Float%20%28double-precision%29) (In%20Decal%20Size :type Vector%202D%20Structure) (In%20Decal%20Region%20Size :type Vector%202D%20Structure :default "(X=256.000000,Y=256.000000)") (In%20Material :type Material%20Interface%20Object%20Reference) (In%20Material%20Parameters :type F%20Blocking%20Decal%20Material%20Parameters%20Structure%20%28by%20ref%29) (In%20Short%20Order :type Integer))
  (bind (_x _y) (Math|Vector2D|BreakVector2D In%20Decal%20Size))
  (Utilities|FlowControl|Sequence
    (:then_0
      ;[1 1 1] Vars
      (bind _returnvalue (Game|ConstructObjectfromClass "/Game/Blueprints/LevelElements/LevelDesignTools/Decals/BP_BlockingDecalData.BP_BlockingDecalData_C"))
      (bind _output_get (LocalVariables|SetNewBlockingDecalData _returnvalue))
      (Utilities|Array|Add (Variables|Default|GetDecals%20List) _output_get)
      (Variables|/Game/Blueprints/LevelElements/LevelDesignTools/Decals/BP_BlockingDecalData.BP_BlockingDecalData_C|SetDecal%20Height (LocalVariables|GetNewBlockingDecalData) In%20Decal%20Height)
      (Variables|/Game/Blueprints/LevelElements/LevelDesignTools/Decals/BP_BlockingDecalData.BP_BlockingDecalData_C|SetDecal%20Size (LocalVariables|GetNewBlockingDecalData) In%20Decal%20Size)
      (Variables|/Game/Blueprints/LevelElements/LevelDesignTools/Decals/BP_BlockingDecalData.BP_BlockingDecalData_C|SetDecal%20Region (LocalVariables|GetNewBlockingDecalData) In%20Decal%20Region%20Size))
    (:then_1
      ;[1 1 1] Component
      (bind _returnvalue_2 (AddComponent|AddSceneComponent false))
      (Variables|/Game/Blueprints/LevelElements/LevelDesignTools/Decals/BP_BlockingDecalData.BP_BlockingDecalData_C|SetDecalRootComponent (LocalVariables|GetNewBlockingDecalData) _returnvalue_2)
      (bind _returnvalue_3 (Game|AddComponentbyClass "/Script/Engine.DecalComponent" true (Math|Transform|MakeTransform "0, 0, 0" "-90.000000, 0, 0")))
      (bind _output_get_2 (Variables|/Game/Blueprints/LevelElements/LevelDesignTools/Decals/BP_BlockingDecalData.BP_BlockingDecalData_C|SetDecalComponent (LocalVariables|GetNewBlockingDecalData) _returnvalue_3))
      (Class|DecalComponent|SetSortOrder _returnvalue_3 In%20Short%20Order)
      (Transformation|SetWorldTransform _output_get_2 (Math|Transform|MakeTransform (Transformation|GetActorLocation) (Math|Rotator|CombineRotators "-90.000000, 0, 0" (Transformation|GetActorRotation)) (* (/ "1.000000,1.000000,1.000000" "128.000000,256.000000,256.000000") (Math|Vector|MakeVector In%20Decal%20Height _y _x))) false false)
      (Transformation|AttachComponentToComponent (Variables|/Game/Blueprints/LevelElements/LevelDesignTools/Decals/BP_BlockingDecalData.BP_BlockingDecalData_C|GetDecalComponent (LocalVariables|GetNewBlockingDecalData)) (Variables|/Game/Blueprints/LevelElements/LevelDesignTools/Decals/BP_BlockingDecalData.BP_BlockingDecalData_C|GetDecalRootComponent (LocalVariables|GetNewBlockingDecalData)) "None" "KeepWorld" "KeepWorld" "KeepWorld" true))
    (:then_2
      ;[1 1 1] Create materials
      (bind _returnvalue_4 (Rendering|Material|CreateDynamicMaterialInstance In%20Material "None" "None" :!class /Script/Engine.KismetMaterialLibrary))
      (Rendering|Components|Decal|SetDecalMaterial (Variables|/Game/Blueprints/LevelElements/LevelDesignTools/Decals/BP_BlockingDecalData.BP_BlockingDecalData_C|GetDecalComponent (LocalVariables|GetNewBlockingDecalData)) _returnvalue_4)
      (Default|SetDecalMaterialParameters (LocalVariables|GetNewBlockingDecalData) In%20Material%20Parameters))
    (:then_3
      (return (LocalVariables|GetNewBlockingDecalData)))))

(fn UpdateDecal
  (CallFunction|UpdateDecalZone)
  (CallFunction|UpdateAllDecalMaterialParameters))

(fn UpdateDecalZone
  (bind _decal_size (Variables|Default|GetDecal%20Size))
  (bind (_x _y) (Math|Vector2D|BreakVector2D _decal_size))
  (Components|Box|SetBoxExtent (Variables|Default|GetDecalZone) (Math|Vector|MakeVector _x _y (Variables|Default|GetDecal%20Height)) true))

(fn UpdateAllDecalMaterialParameters
  (for _array_element (Variables|Default|GetDecals%20List)
    (Default|UpdateDecalMaterialParameters _array_element)))