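; BP_SimpleBlockingDecal is a level design tool actor that places a single configurable decal in the level.
; Its construction script runs the parent's script, then calls CreateDecal with the configured height, material, material parameters and sort order.
; The decal size is scaled by the actor's X and Y scale, while the region size keeps the unscaled value.
; The event graph has no active logic.
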(event EventBeginPlay)

(event EventTick
  (params (DeltaSeconds :type Float%20%28single-precision%29)))

(fn ConstructionScript
  (bind _returnvalue (Transformation|GetActorScale3D))
  (bind _decal_size (Variables|Default|GetDecal%20Size))
  (bind (_x _y) (Math|Vector|BreakVector _returnvalue))
  (|CallParentFunction)
  (CallFunction|CreateDecal (Variables|Default|GetDecal%20Height) (* _decal_size (Math|Vector2D|MakeVector2D _x _y)) _decal_size (Variables|Default|GetDecalMaterial) (Variables|Default|GetDecal%20Parameters) (Variables|Default|GetDecals%20Short%20Order)))