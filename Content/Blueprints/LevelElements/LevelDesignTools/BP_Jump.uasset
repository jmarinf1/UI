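; BP_Jump is a level design tool for a jumping gap in a high or low variant, teleporting player 0 between its two sides.
; The construction script uses HighJump to hide the other variant's mesh and markers, changing visibility only.
; The right trigger sends the player to the high or low right point by that flag.
; Both left triggers send the player to the shared left point, only when HighJump is true.
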(event OnComponentBeginOverlap(TV_JumpRight)
  (params (OverlappedComponent :type Primitive%20Component%20Object%20Reference) (OtherActor :type Actor%20Object%20Reference) (OtherComp :type Primitive%20Component%20Object%20Reference) (OtherBodyIndex :type Integer) (bFromSweep :type Boolean) (SweepResult :type Hit%20Result%20Structure%20%28by%20ref%29))
  ;[1 1 1] Check Which Jump is Active to then teleport player to correct 'Right'
  (if (Variables|JumpHeight|GetHighJump)
    ;[1 1 1] Teleport PPlayer Hight
    (Transformation|Teleport (Game|GetPlayerCharacter 0) (Transformation|GetWorldLocation (Variables|Default|GetTP_Right_High)) (Transformation|GetWorldRotation (Variables|Default|GetTP_Right_High)))
    (else
      (|TeleportPlayerRightLow))))

(event OnComponentBeginOverlap(TV_LeftHigh)
  (params (OverlappedComponent :type Primitive%20Component%20Object%20Reference) (OtherActor :type Actor%20Object%20Reference) (OtherComp :type Primitive%20Component%20Object%20Reference) (OtherBodyIndex :type Integer) (bFromSweep :type Boolean) (SweepResult :type Hit%20Result%20Structure%20%28by%20ref%29))
  ;[1 1 1] If Active Send Players to the left
  (if (Variables|JumpHeight|GetHighJump)
    (|TeleportPlayerLeft_2)))

(event OnComponentBeginOverlap(TV_LeftLow)
  (params (OverlappedComponent :type Primitive%20Component%20Object%20Reference) (OtherActor :type Actor%20Object%20Reference) (OtherComp :type Primitive%20Component%20Object%20Reference) (OtherBodyIndex :type Integer) (bFromSweep :type Boolean) (SweepResult :type Hit%20Result%20Structure%20%28by%20ref%29))
  ;[1 1 1] If Active Send Players to the left
  (if (Variables|JumpHeight|GetHighJump)
    (|TeleportPlayerLeft)))

(fn ConstructionScript
  (if (Variables|JumpHeight|GetHighJump)
    (|HideLowJump)
    (else
      (|HideHighJump))))