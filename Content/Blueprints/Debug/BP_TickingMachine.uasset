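; BP_TickingMachine is a debug actor that periodically reports which actors are within range of it.
; Tick accumulates delta time and resets it whenever it passes RefreshTime.
; Each interval runs a zero-length multi sphere trace on the Visibility channel at the actor's location, using Range as radius and ignoring itself.
; The trace is drawn briefly, and each hit actor's display name is printed to screen.
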(event EventBeginPlay)

(event Collision|EventActorBeginOverlap
  (params (OtherActor :type Actor%20Object%20Reference)))

(event EventTick
  (params (DeltaSeconds :type Float%20%28single-precision%29))
  (bind _returnvalue (Transformation|GetActorLocation))
  (bind _output_get (Variables|Default|SetTimeClock (+ DeltaSeconds (Variables|Default|GetTimeClock))))
  (if (> _output_get (Variables|Default|GetRefreshTime))
    (Variables|Default|SetTimeClock 0.0)
    (bind _outhits (Collision|MultiSphereTraceByChannel _returnvalue _returnvalue (Variables|Default|GetRange) "TraceTypeQuery1" false (Utilities|Array|MakeArray self) "ForDuration" true "(R=1.000000,G=0.000000,B=0.000000,A=1.000000)" "(R=0.000000,G=1.000000,B=0.000000,A=1.000000)" 1.5))
    (bind _array_element (Utilities|Array|ForEachLoopwithBreak _outhits)
      (:LoopBody
        (Development|PrintString (Utilities|GetDisplayName (.HitActor (Collision|BreakHitResult _array_element))))))))

(fn ConstructionScript)